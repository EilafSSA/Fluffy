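; Stats component for the virtual pet Fluffy, tracking hunger, boredom, dirtyness and drowsyness, with happiness as their average.
; A looping one-second timer drains each stat, mostly by randomized amounts, and updates state flags.
; Number and letter keys trigger eating, showering, sleeping or playing, which swap Fluffy's plane material, play audio and refill the stat after a delay.
; On BeginPlay it initializes stats and adds a bars widget to Fluffy's HUD.
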(event EventBeginPlay
  (Utilities|FlowControl|Sequence
    (:then_0
      ;[0.15 0.15 0.15 0.5] character stuff
      ;;[0.15 0.15 0.15 0.5] initalizing character
      (bind _aspawn (Utilities|Casting|CastToPawn (Components|GetOwner)))
      (Variables|DoNotEdit|SetOwneing%20Character%20ref _aspawn))
    (:then_1
      ;;[0.15 0.15 0.15 0.5] Validating Character
      (bind _owneing_character_ref (Variables|DoNotEdit|GetOwneing%20Character%20ref)
        (:then
          (bind _asbp_fluffy (Utilities|Casting|CastToBP_Fluffy _owneing_character_ref))
          (Variables|Default|SetAs%20BP%20Fluffy _asbp_fluffy))
        (:else)))
    (:then_2
      (initialize|InitializingStats))
    (:then_3
      (initialize|InitTimerHandling))
    (:then_4
      (Utilities|FlowControl|Delay 1.0)
      (UI|AddFoodBarUItoMainHUD))))

(event Input|KeyboardEvents|X
  (params (Key :type Key%20Structure :default "None"))
  (bind _as_bp_fluffy (Variables|Default|GetAs%20BP%20Fluffy))
  (bind _audio_showering (Variables|/Game/Fluffy/BP_Fluffy.BP_Fluffy_C|GetAudio_Showering _as_bp_fluffy))
  ;[0.03412 0.15 0.1244 0.5] Showering
  (:Pressed
    (Variables|Action|SetIsShowering? true)
    (Utilities|FlowControl|Sequence
      (:then_0
        (Rendering|Material|SetMaterial (Variables|/Game/Fluffy/BP_Fluffy.BP_Fluffy_C|GetPlane (Variables|Default|GetAs%20BP%20Fluffy)) 0 "/Game/Fluffy/FluffyTEXTURES/M_FluffyShower.M_FluffyShower")
        (Utilities|FlowControl|Delay 1.0)
        (Variables|DoNotEdit--CurrentStat|SetCurrent%20Dirtyness (+ (Variables|DoNotEdit--CurrentStat|GetCurrent%20Dirtyness) 1e+02))
        (Variables|Action|SetIsShowering? false)
        (Audio|Components|Audio|Stop _audio_showering))
      (:then_1
        (Audio|Components|Audio|Play _audio_showering 0.0)))))

(event Input|KeyboardEvents|3
  (params (Key :type Key%20Structure :default "None"))
  (bind _returnvalue (Math|Random|RandomFloatinRange 5.0 8.0))
  (bind _as_bp_fluffy (Variables|Default|GetAs%20BP%20Fluffy))
  (bind _as_bp_fluffy_2 (Variables|Default|GetAs%20BP%20Fluffy))
  (bind _plane (Variables|/Game/Fluffy/BP_Fluffy.BP_Fluffy_C|GetPlane _as_bp_fluffy_2))
  (bind _audio_snoring (Variables|/Game/Fluffy/BP_Fluffy.BP_Fluffy_C|GetAudio_Snoring _as_bp_fluffy))
  ;[0.0225 0.05058 0.15 0.5] Sleeping
  (:Pressed
    (Variables|Action|SetIsSleeping? true)
    (Utilities|FlowControl|Sequence
      (:then_0
        (Variables|Default|SetSleepingDuration _returnvalue))
      (:then_1
        (Rendering|Material|SetMaterial _plane 0 "/Game/Fluffy/FluffyTEXTURES/M_FluffySleepStart.M_FluffySleepStart")
        (Utilities|FlowControl|Delay 1.5)
        (Rendering|Material|SetMaterial _plane 0 "/Game/Fluffy/FluffyTEXTURES/M_FluffySleepStart1.M_FluffySleepStart1")
        (Utilities|FlowControl|Delay _returnvalue)
        (Variables|Action|SetIsSleeping? false)
        (Variables|DoNotEdit--CurrentStat|SetCurrent%20Drowsyness (+ (Variables|DoNotEdit--CurrentStat|GetCurrent%20Drowsyness) 1e+02))
        (Audio|Components|Audio|Stop _audio_snoring))
      (:then_2
        (Audio|Components|Audio|Play _audio_snoring 0.0)))))

(event Input|KeyboardEvents|C
  (params (Key :type Key%20Structure :default "None"))
  (bind _returnvalue (Math|Random|RandomFloatinRange 5.0 8.0))
  (bind _as_bp_fluffy (Variables|Default|GetAs%20BP%20Fluffy))
  (bind _as_bp_fluffy_2 (Variables|Default|GetAs%20BP%20Fluffy))
  (bind _plane (Variables|/Game/Fluffy/BP_Fluffy.BP_Fluffy_C|GetPlane _as_bp_fluffy_2))
  (bind _audio_snoring (Variables|/Game/Fluffy/BP_Fluffy.BP_Fluffy_C|GetAudio_Snoring _as_bp_fluffy))
  ;[0.0225 0.05058 0.15 0.5] Sleeping
  (:Pressed
    (Variables|Action|SetIsSleeping? true)
    (Utilities|FlowControl|Sequence
      (:then_0
        (Variables|Default|SetSleepingDuration _returnvalue))
      (:then_1
        (Rendering|Material|SetMaterial _plane 0 "/Game/Fluffy/FluffyTEXTURES/M_FluffySleepStart.M_FluffySleepStart")
        (Utilities|FlowControl|Delay 1.5)
        (Rendering|Material|SetMaterial _plane 0 "/Game/Fluffy/FluffyTEXTURES/M_FluffySleepStart1.M_FluffySleepStart1")
        (Utilities|FlowControl|Delay _returnvalue)
        (Variables|Action|SetIsSleeping? false)
        (Variables|DoNotEdit--CurrentStat|SetCurrent%20Drowsyness (+ (Variables|DoNotEdit--CurrentStat|GetCurrent%20Drowsyness) 1e+02))
        (Audio|Components|Audio|Stop _audio_snoring))
      (:then_2
        (Audio|Components|Audio|Play _audio_snoring 0.0)))))

(event Input|KeyboardEvents|4
  (params (Key :type Key%20Structure :default "None"))
  (bind _as_bp_fluffy (Variables|Default|GetAs%20BP%20Fluffy))
  (bind _audio_playing (Variables|/Game/Fluffy/BP_Fluffy.BP_Fluffy_C|GetAudio_Playing _as_bp_fluffy))
  ;[0.1462 0.05087 0.15 0.5] Playing
  (:Pressed
    (Variables|Action|SetIsPlaying? true)
    (Utilities|FlowControl|Sequence
      (:then_0
        (Rendering|Material|SetMaterial (Variables|/Game/Fluffy/BP_Fluffy.BP_Fluffy_C|GetPlane (Variables|Default|GetAs%20BP%20Fluffy)) 0 "/Game/Fluffy/FluffyTEXTURES/M_FluffyPlay.M_FluffyPlay")
        (Utilities|FlowControl|Delay 1.0)
        (Variables|DoNotEdit--CurrentStat|SetCurrent%20Boredom (+ (Variables|DoNotEdit--CurrentStat|GetCurrent%20Boredom) 1e+02))
        (Variables|Action|SetIsPlaying? false)
        (Audio|Components|Audio|Stop _audio_playing))
      (:then_1
        (Audio|Components|Audio|Play _audio_playing 0.0)))))

(event Input|KeyboardEvents|V
  (params (Key :type Key%20Structure :default "None"))
  (bind _as_bp_fluffy (Variables|Default|GetAs%20BP%20Fluffy))
  (bind _audio_playing (Variables|/Game/Fluffy/BP_Fluffy.BP_Fluffy_C|GetAudio_Playing _as_bp_fluffy))
  ;[0.1462 0.05087 0.15 0.5] Playing
  (:Pressed
    (Variables|Action|SetIsPlaying? true)
    (Utilities|FlowControl|Sequence
      (:then_0
        (Rendering|Material|SetMaterial (Variables|/Game/Fluffy/BP_Fluffy.BP_Fluffy_C|GetPlane (Variables|Default|GetAs%20BP%20Fluffy)) 0 "/Game/Fluffy/FluffyTEXTURES/M_FluffyPlay.M_FluffyPlay")
        (Utilities|FlowControl|Delay 1.0)
        (Variables|DoNotEdit--CurrentStat|SetCurrent%20Boredom (+ (Variables|DoNotEdit--CurrentStat|GetCurrent%20Boredom) 1e+02))
        (Variables|Action|SetIsPlaying? false)
        (Audio|Components|Audio|Stop _audio_playing))
      (:then_1
        (Audio|Components|Audio|Play _audio_playing 0.0)))))

(event Input|KeyboardEvents|1
  (params (Key :type Key%20Structure :default "None"))
  (bind _as_bp_fluffy (Variables|Default|GetAs%20BP%20Fluffy))
  (bind _audio_eating (Variables|/Game/Fluffy/BP_Fluffy.BP_Fluffy_C|GetAudio_Eating _as_bp_fluffy))
  ;[0.15 0.07011 0.02302 0.5] Feeding
  (:Pressed
    (Variables|Action|SetIsEating? true)
    (Utilities|FlowControl|Sequence
      (:then_0
        (Rendering|Material|SetMaterial (Variables|/Game/Fluffy/BP_Fluffy.BP_Fluffy_C|GetPlane (Variables|Default|GetAs%20BP%20Fluffy)) 0 "/Game/Fluffy/FluffyTEXTURES/M_FluffyEat.M_FluffyEat")
        (Utilities|FlowControl|Delay 1.0)
        (Variables|DoNotEdit--CurrentStat|SetCurrent%20Hunger (+ (Variables|DoNotEdit--CurrentStat|GetCurrent%20Hunger) 1e+02))
        (Variables|Action|SetIsEating? false)
        (Audio|Components|Audio|Stop _audio_eating))
      (:then_1
        (Audio|Components|Audio|Play _audio_eating 0.0)))))

(event Input|KeyboardEvents|Z
  (params (Key :type Key%20Structure :default "None"))
  (bind _as_bp_fluffy (Variables|Default|GetAs%20BP%20Fluffy))
  (bind _audio_eating (Variables|/Game/Fluffy/BP_Fluffy.BP_Fluffy_C|GetAudio_Eating _as_bp_fluffy))
  ;[0.15 0.07011 0.02302 0.5] Feeding
  (:Pressed
    (Variables|Action|SetIsEating? true)
    (Utilities|FlowControl|Sequence
      (:then_0
        (Rendering|Material|SetMaterial (Variables|/Game/Fluffy/BP_Fluffy.BP_Fluffy_C|GetPlane (Variables|Default|GetAs%20BP%20Fluffy)) 0 "/Game/Fluffy/FluffyTEXTURES/M_FluffyEat.M_FluffyEat")
        (Utilities|FlowControl|Delay 1.0)
        (Variables|DoNotEdit--CurrentStat|SetCurrent%20Hunger (+ (Variables|DoNotEdit--CurrentStat|GetCurrent%20Hunger) 1e+02))
        (Variables|Action|SetIsEating? false)
        (Audio|Components|Audio|Stop _audio_eating))
      (:then_1
        (Audio|Components|Audio|Play _audio_eating 0.0)))))

(event Input|KeyboardEvents|2
  (params (Key :type Key%20Structure :default "None"))
  (bind _as_bp_fluffy (Variables|Default|GetAs%20BP%20Fluffy))
  (bind _audio_showering (Variables|/Game/Fluffy/BP_Fluffy.BP_Fluffy_C|GetAudio_Showering _as_bp_fluffy))
  ;[0.03412 0.15 0.1244 0.5] Showering
  (:Pressed
    (Variables|Action|SetIsShowering? true)
    (Utilities|FlowControl|Sequence
      (:then_0
        (Rendering|Material|SetMaterial (Variables|/Game/Fluffy/BP_Fluffy.BP_Fluffy_C|GetPlane (Variables|Default|GetAs%20BP%20Fluffy)) 0 "/Game/Fluffy/FluffyTEXTURES/M_FluffyShower.M_FluffyShower")
        (Utilities|FlowControl|Delay 1.0)
        (Variables|DoNotEdit--CurrentStat|SetCurrent%20Dirtyness (+ (Variables|DoNotEdit--CurrentStat|GetCurrent%20Dirtyness) 1e+02))
        (Variables|Action|SetIsShowering? false)
        (Audio|Components|Audio|Stop _audio_showering))
      (:then_1
        (Audio|Components|Audio|Play _audio_showering 0.0)))))

(fn GetCurrentDrowsyness
  (return (Variables|DoNotEdit--CurrentStat|GetCurrent%20Drowsyness)))

(fn GetCurrentBored
  (return (Variables|StartingStats|GetStarting%20Boredom)))

(fn GetCurrentDirty
  (return (Variables|DoNotEdit--CurrentStat|GetCurrent%20Dirtyness)))

(fn GetCurrentFood
  (return (Variables|DoNotEdit--CurrentStat|GetCurrent%20Hunger)))

(fn OnRepCurrentHunger)

(fn OnRepCurrentBoredom)

(fn OnRepCurrentDirtyness)

(fn OnRepCurrentDrowsyness)

(fn OnRepCurrentHappiness)

(fn DecreasingStats
  (params (Amount%20to%20decrease :type Float%20%28double-precision%29))
  (Utilities|FlowControl|Sequence
    (:then_0
      ;[0.1447 0.15 0.04688 0.5] HUNGER
      (if (> (Math|Float|Clamp(Float) (- (Variables|DoNotEdit--CurrentStat|GetCurrent%20Hunger) (+ Amount%20to%20decrease (Math|Random|RandomFloatinRange 0.0 2.0))) 0.0 (Variables|MaxStats|GetMax%20Hunger)) 0.0)
        (Variables|DoNotEdit--CurrentStat|SetCurrent%20Hunger (Math|Float|Clamp(Float) (- (Variables|DoNotEdit--CurrentStat|GetCurrent%20Hunger) (+ Amount%20to%20decrease (Math|Random|RandomFloatinRange 0.0 2.0))) 0.0 (Variables|MaxStats|GetMax%20Hunger)))
        (Variables|DoNotEdit|SetIsStarving? true)
        (Development|PrintText "hungrynot")
        (else
          (Variables|DoNotEdit--CurrentStat|SetCurrent%20Hunger 0.0)
          (Variables|DoNotEdit|SetIsStarving? false)
          (Development|PrintText "starveeeed"))))
    (:then_1
      ;[0.05624 0.1121 0.15 0.5] BOREDOM
      (if (> (Math|Float|Clamp(Float) (- (Variables|DoNotEdit--CurrentStat|GetCurrent%20Boredom) (+ (Math|Random|RandomFloatinRange 0.0 2.0) Amount%20to%20decrease)) 0.0 (Variables|MaxStats|GetMax%20Boredom)) 0.0)
        (Variables|DoNotEdit--CurrentStat|SetCurrent%20Boredom (Math|Float|Clamp(Float) (- (Variables|DoNotEdit--CurrentStat|GetCurrent%20Boredom) (+ (Math|Random|RandomFloatinRange 0.0 2.0) Amount%20to%20decrease)) 0.0 (Variables|MaxStats|GetMax%20Boredom)))
        (Variables|DoNotEdit|SetIsBored? true)
        (Development|PrintText "NotBored")
        (else
          (Variables|DoNotEdit--CurrentStat|SetCurrent%20Boredom 0.0)
          (Variables|DoNotEdit|SetIsBored? false)
          (Development|PrintText "BORED!"))))
    (:then_2
      ;[0.15 0.05669 0.0524 0.5] DIRTYNESS
      (if (> (Math|Float|Clamp(Float) (- (Variables|DoNotEdit--CurrentStat|GetCurrent%20Dirtyness) (+ (Math|Random|RandomFloatinRange 0.0 1.0) Amount%20to%20decrease)) 0.0 (Variables|MaxStats|GetMax%20Dirtyness)) 0.0)
        (Variables|DoNotEdit--CurrentStat|SetCurrent%20Dirtyness (Math|Float|Clamp(Float) (- (Variables|DoNotEdit--CurrentStat|GetCurrent%20Dirtyness) (+ (Math|Random|RandomFloatinRange 0.0 1.0) Amount%20to%20decrease)) 0.0 (Variables|MaxStats|GetMax%20Dirtyness)))
        (Variables|DoNotEdit|SetIsDirty? true)
        (Development|PrintText "Clean")
        (else
          (Variables|DoNotEdit--CurrentStat|SetCurrent%20Dirtyness 0.0)
          (Variables|DoNotEdit|SetIsDirty? false)
          (Development|PrintText "Dirty"))))
    (:then_3
      ;[0.15 0.06794 0.11 0.5] DROWSYNESS
      (if (> (Math|Float|Clamp(Float) (- (Variables|DoNotEdit--CurrentStat|GetCurrent%20Drowsyness) Amount%20to%20decrease) 0.0 (Variables|MaxStats|GetMax%20Drowsyness)) 0.0)
        (Variables|DoNotEdit--CurrentStat|SetCurrent%20Drowsyness (Math|Float|Clamp(Float) (- (Variables|DoNotEdit--CurrentStat|GetCurrent%20Drowsyness) Amount%20to%20decrease) 0.0 (Variables|MaxStats|GetMax%20Drowsyness)))
        (Variables|DoNotEdit|SetIsSleepy? true)
        (Development|PrintText "wellrested")
        (else
          (Variables|DoNotEdit--CurrentStat|SetCurrent%20Drowsyness 0.0)
          (Variables|DoNotEdit|SetIsSleepy? false)
          (Development|PrintText "Sleepy"))))
    (:then_4
      ;[0.1447 0.15 0.04688 0.5] HAPPINESS
      (Variables|DoNotEdit--CurrentStat|SetCurrent%20Happiness (/ (+ (Variables|DoNotEdit--CurrentStat|GetCurrent%20Hunger) (Variables|DoNotEdit--CurrentStat|GetCurrent%20Boredom) (Variables|DoNotEdit--CurrentStat|GetCurrent%20Dirtyness) (Variables|DoNotEdit--CurrentStat|GetCurrent%20Drowsyness)) 4)))))

(fn TimerFunctionDecreaseStats
  (Stats|DecreasingStats (Variables|Timers|GetAmount%20To%20Decrease)))

(fn AddFoodBarUItoMainHUD
  (bind _returnvalue (UserInterface|CreateWidget "/Game/Fluffy/StatSystem/HUD_Widgets/WBP_Bars_U1.WBP_Bars_U1_C" 0 self))
  (bind _as_bp_fluffy (Variables|Default|GetAs%20BP%20Fluffy)
    (:then
      (bind _returnvalue_2 (Class|CanvasPanel|AddChildtoCanvas (Variables|/Game/Fluffy/StatSystem/HUD_Widgets/WBP_MainHUD.WBP_MainHUD_C|GetMainHUD_Canvas (Default|GetMainHUD _as_bp_fluffy)) _returnvalue))
      (Class|CanvasPanelSlot|SetAutoSize _returnvalue_2 true)
      (Class|CanvasPanelSlot|SetAnchors _returnvalue_2))
    (:else)))

(fn InitializingStats
  (Utilities|FlowControl|Sequence
    (:then_0
      (bind _output_get (Variables|DoNotEdit--CurrentStat|SetCurrent%20Hunger (Variables|StartingStats|GetStarting%20Hunger)))
      (Variables|MaxStats|SetMax%20Hunger _output_get))
    (:then_1
      (bind _output_get_2 (Variables|DoNotEdit--CurrentStat|SetCurrent%20Boredom (Variables|StartingStats|GetStarting%20Boredom)))
      (Variables|MaxStats|SetMax%20Boredom _output_get_2))
    (:then_2
      (bind _output_get_3 (Variables|DoNotEdit--CurrentStat|SetCurrent%20Dirtyness (Variables|StartingStats|GetStarting%20Dirtyness)))
      (Variables|MaxStats|SetMax%20Dirtyness _output_get_3))
    (:then_3
      (bind _output_get_4 (Variables|DoNotEdit--CurrentStat|SetCurrent%20Drowsyness (Variables|StartingStats|GetStarting%20Drowsyness)))
      (Variables|MaxStats|SetMax%20Drowsyness _output_get_4))))

(fn InitTimerHandling
  (bind _returnvalue (Utilities|Time|SetTimerbyFunctionName 0 "TimerFunction_DecreaseStats" 1.0 true))
  (Variables|Timers|SetTimer_Hunger _returnvalue))