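; Blueprint for Fluffy, a virtual pet shown on a plane that wanders along the room's X axis and owns the main HUD.
; BeginPlay activates the BPFluffyStats component, starts the wander loop, and creates the WBP_MainHUD widget, exposed through GetMainHUD.
; Each loop eases the plane to a random position with a move material, then picks a happy-idle or eat material by testing CurrentHappiness against a random threshold, and repeats after a random delay.
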(event EventBeginPlay
  (bind _plane (Variables|Default|GetPlane))
  (bind _plane_2 (Variables|Default|GetPlane))
  (Utilities|FlowControl|Sequence
    (:then_0
      (Components|Activation|Activate (Variables|Default|GetBP_Fluffy_Stats) false))
    (:then_1
      ;[0.15 0.15 0.15 0.5] fluffy movement
      (Rendering|Material|SetMaterial _plane 0 "/Game/Fluffy/FluffyTEXTURES/M_FluffyMove.M_FluffyMove" :!label _label)
      (Components|MoveComponentTo _plane (Math|Vector|MakeVector (Math|Random|RandomFloatinRange (Variables|DoNotEdit|GetMax%20Room%20X) (Variables|DoNotEdit|GetMin%20Room%20X)) 0.0 3e+01) "0.000000,0.000000,90.000000" true true (Math|Random|RandomFloatinRange 1.0 2.0) false)
      (if (> (Variables|/Game/Fluffy/StatSystem/BP_Fluffy_Stats.BP_Fluffy_Stats_C|GetCurrent%20Happiness (Variables|Default|GetBP_Fluffy_Stats)) (Math|Random|RandomFloatinRange 45.0 1e+02))
        (Rendering|Material|SetMaterial _plane_2 0 "/Game/Fluffy/FluffyTEXTURES/M_FluffyIdle_Happy.M_FluffyIdle_Happy")
        (else
          (Rendering|Material|SetMaterial _plane_2 0 "/Game/Fluffy/FluffyTEXTURES/M_FluffyEat.M_FluffyEat")))
      (Utilities|FlowControl|Delay (Math|Random|RandomFloatinRange 2.0 5.0))
      (Utilities|FlowControl|ForLoopwithBreak 0 0
        (:LoopBody
          (goto _label))))
    (:then_3
      ;[0.15 0.15 0.15 0.5] spawning viewport from pawn
      (bind _returnvalue (UserInterface|CreateWidget "/Game/Fluffy/StatSystem/HUD_Widgets/WBP_MainHUD.WBP_MainHUD_C"))
      (bind _output_get (Variables|Default|SetMainHUD_ref _returnvalue))
      (UserInterface|Viewport|AddtoViewport _output_get 0))))

(fn ConstructionScript)

(fn GetMainHUD
  (bind _mainhud_ref (Variables|Default|GetMainHUD_ref)
    (:then
      (return _mainhud_ref))
    (:else
      (return 0))))